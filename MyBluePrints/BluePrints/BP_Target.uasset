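; BP_Target is a destructible target actor that counts toward level completion when eliminated.
; ApplyTargetDamage subtracts DamageAmount from TargetHealth and pushes the result to its TargetHealthBar widget component, which BeginPlay also initializes.
; At zero health or below, it increments TargetsEliminated on the player's BP_FirstPersonCharacter, calls CheckLevelComplete there, then destroys itself.
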(event `ApplyTargetDamage`
  ;[1 1 1] Apply Damage to Target and Display Current Health
  (bind _output_get (set `self.TargetHealth` (- (`self.TargetHealth`) (`self.DamageAmount`))))
  (bind _astarget_health_bar (cast `/Game/UserInterface/TargetHealthBar` (`WidgetComponent.GetUserWidgetObject` (`self.HealthBarWidget`))))
  (`/Game/UserInterface/TargetHealthBar.UpdateHealthBar` _astarget_health_bar _output_get)
  (if (<= _output_get 0)
    (bind _asbp_first_person_character (cast `/Game/FirstPerson/Blueprints/BP_FirstPersonCharacter` (`GameplayStatics.GetPlayerCharacter` 0)))
    (bind _result (`/Engine/EditorBlueprintResources/StandardMacros.IncrementInt` (`/Game/FirstPerson/Blueprints/BP_FirstPersonCharacter.TargetsEliminated` _asbp_first_person_character))
      (:`  `
        (set `/Game/FirstPerson/Blueprints/BP_FirstPersonCharacter.TargetsEliminated` _result _asbp_first_person_character)
        (`/Game/FirstPerson/Blueprints/BP_FirstPersonCharacter.CheckLevelComplete` _asbp_first_person_character)
        (`self.K2_DestroyActor`)))))

(event `self.ReceiveBeginPlay`
  ;[1 1 1] Start all Health Bars at 100%
  (bind _astarget_health_bar (cast `/Game/UserInterface/TargetHealthBar` (`WidgetComponent.GetUserWidgetObject` (`self.HealthBarWidget`))))
  (`/Game/UserInterface/TargetHealthBar.UpdateHealthBar` _astarget_health_bar (`self.TargetHealth`)))

(fn `UserConstructionScript`)